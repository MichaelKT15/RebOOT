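; Final terminal actor that checks whether three terminals have been activated when the player uses it.
; TerminalPressed, with no caller in this graph, increments the activation count and reveals the matching light for each of the first three.
; The trigger overlap toggles input and a Gate, so pressing E in range plays a power-up sound at three or more activations, otherwise a power-fail sound.
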(event `Key|E`
  (params (Key :type "Key Structure"))
  (:`Pressed`
    (`/Engine/EditorBlueprintResources/StandardMacros.Gate` true :!label _label
      (:`Exit`
        (if (>= (`self.TerminalsActivated`) 3)
          (`GameplayStatics.PlaySound2D` "/Game/Sounds/powerupeffect.powerupeffect" 0.2 1.0 0.0 null null)
          (else
            (`GameplayStatics.PlaySound2D` "/Game/Sounds/powerfaileffect.powerfaileffect" 0.2 1.0 0.0 null null)))))))

(event `self.Trigger.OnComponentBeginOverlap`
  (params (OverlappedComponent :type "PrimitiveComponent Object Reference") (OtherActor :type "Actor Object Reference") (OtherComp :type "PrimitiveComponent Object Reference") (OtherBodyIndex :type Integer) (bFromSweep :type Boolean) (SweepResult :type "HitResult Structure (by ref)"))
  (`self.EnableInput` (`GameplayStatics.GetPlayerController` 0))
  (goto _label :!via `Open`))

(event `self.Trigger.OnComponentEndOverlap`
  (params (OverlappedComponent :type "PrimitiveComponent Object Reference") (OtherActor :type "Actor Object Reference") (OtherComp :type "PrimitiveComponent Object Reference") (OtherBodyIndex :type Integer))
  (`self.DisableInput` (`GameplayStatics.GetPlayerController` 0) null)
  (goto _label :!via `Close`))

(fn `TerminalPressed`
  (bind _result (`/Engine/EditorBlueprintResources/StandardMacros.IncrementInt` (`self.TerminalsActivated`))
    (:`  `
      (bind _output_get (set `self.TerminalsActivated` _result))
      (switch `int` _output_get
        (:`1`
          (`SceneComponent.SetVisibility` (`self.RectLight`) true false))
        (:`2`
          (`SceneComponent.SetVisibility` (`self.RectLight2`) true false))
        (:`3`
          (`SceneComponent.SetVisibility` (`self.ActiveLight1`) true false))))))

(fn `UserConstructionScript`)