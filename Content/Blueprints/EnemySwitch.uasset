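; EnemySwitch is an interactable switch that flags two referenced Bot_AI enemies to change their path.
; Overlapping its Trigger enables player input, shows the CanActivate indicator and opens a Gate, and leaving reverses all three.
; While the Gate is open, pressing E plays a click sound and sets PathChange to true on both bots, provided both casts succeed.
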(event `Key|E`
  (params (Key :type "Key Structure"))
  (:`Pressed`
    (`/Engine/EditorBlueprintResources/StandardMacros.Gate` true :!label _label
      (:`Exit`
        (`GameplayStatics.PlaySound2D` "/Engine/VREditor/Sounds/UI/Click_on_Button.Click_on_Button" 1.0 1.0 0.0 null null)
        (bind _asbot_ai (cast `/Game/Blueprints/Bot_AI` (`self.MyOtherBot`)))
        (bind _asbot_ai_2 (cast `/Game/Blueprints/Bot_AI` (`self.MyBot`)))
        (set `/Game/Blueprints/Bot_AI.PathChange` true _asbot_ai_2)
        (set `/Game/Blueprints/Bot_AI.PathChange` true _asbot_ai)))))

(event `self.Trigger.OnComponentBeginOverlap`
  (params (OverlappedComponent :type "PrimitiveComponent Object Reference") (OtherActor :type "Actor Object Reference") (OtherComp :type "PrimitiveComponent Object Reference") (OtherBodyIndex :type Integer) (bFromSweep :type Boolean) (SweepResult :type "HitResult Structure (by ref)"))
  (`self.EnableInput` (`GameplayStatics.GetPlayerController` 0))
  (`SceneComponent.SetVisibility` (`self.CanActivate`) true false)
  (goto _label :!via `Open`))

(event `self.Trigger.OnComponentEndOverlap`
  (params (OverlappedComponent :type "PrimitiveComponent Object Reference") (OtherActor :type "Actor Object Reference") (OtherComp :type "PrimitiveComponent Object Reference") (OtherBodyIndex :type Integer))
  (`self.DisableInput` (`GameplayStatics.GetPlayerController` 0))
  (`SceneComponent.SetVisibility` (`self.CanActivate`) false false)
  (goto _label :!via `Close`))

(fn `UserConstructionScript`)