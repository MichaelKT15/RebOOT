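; DoorTerminal is an interactable terminal that opens one linked door and closes another when E is pressed.
; Entering its Trigger volume enables input for player 0, shows the CanActivate indicator and opens a Gate; leaving reverses all three.
; While the Gate is open, pressing E plays a click sound, calls DoorOpen on MyDoor and calls DoorClose on MyOtherDoor.
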(event `Key|E`
  (params (Key :type "Key Structure"))
  (:`Pressed`
    (`/Engine/EditorBlueprintResources/StandardMacros.Gate` true :!label _label
      (:`Exit`
        (`GameplayStatics.PlaySound2D` "/Engine/VREditor/Sounds/UI/Click_on_Button.Click_on_Button" 1.0 1.0 0.0 null null)
        (`/Game/Blueprints/Door.DoorOpen` (`self.MyDoor`))
        (`/Game/Blueprints/Door.DoorClose` (`self.My Other Door`))))))

(event `self.Trigger.OnComponentBeginOverlap`
  (params (OverlappedComponent :type "PrimitiveComponent Object Reference") (OtherActor :type "Actor Object Reference") (OtherComp :type "PrimitiveComponent Object Reference") (OtherBodyIndex :type Integer) (bFromSweep :type Boolean) (SweepResult :type "HitResult Structure (by ref)"))
  (`self.EnableInput` (`GameplayStatics.GetPlayerController` 0))
  (`SceneComponent.SetVisibility` (`self.CanActivate`) true false)
  (goto _label :!via `Open`))

(event `self.Trigger.OnComponentEndOverlap`
  (params (OverlappedComponent :type "PrimitiveComponent Object Reference") (OtherActor :type "Actor Object Reference") (OtherComp :type "PrimitiveComponent Object Reference") (OtherBodyIndex :type Integer))
  (`self.DisableInput` (`GameplayStatics.GetPlayerController` 0))
  (`SceneComponent.SetVisibility` (`self.CanActivate`) false false)
  (goto _label :!via `Close`))

(fn `UserConstructionScript`)